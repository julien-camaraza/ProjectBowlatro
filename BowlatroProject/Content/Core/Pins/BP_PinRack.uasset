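; Bowling pin rack actor that spawns, tracks, counts and clears the pins of a layout.
; SpawnPinsFromLayout replaces existing pins with BP_PinActors placed relative to the rack, each initialized from its PinDef.
; Count queries report total, knocked and newly knocked pins, with variants limited to pins contributing to standard bowling rules.
; GetNewlyKnockedPinCount also flags pins CountAsKnocked, preventing recounts and marking them for RemoveKnockedDownPins to destroy.
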(event EventBeginPlay)

(event Collision|EventActorBeginOverlap
  (params (OtherActor :type Actor%20Object%20Reference)))

(event EventTick
  (params (DeltaSeconds :type Float%20%28single-precision%29)))

(fn ConstructionScript)

(fn SpawnPinsfromLayout
  (params (PinLayoutToSpawn :type PDA%20Pin%20Layout%20Def%20Object%20Reference))
  (HandlePins|ClearExistingPins)
  (Utilities|IsValid PinLayoutToSpawn
    (:Is%20Valid
      (for _array_element (Variables|/Game/Data/PinLayouts/PDA_PinLayoutDef.PDA_PinLayoutDef_C|GetPinSpawns PinLayoutToSpawn)
        (bind _returnvalue (Game|SpawnActorfromClass "/Game/Core/Pins/BP_PinActor.BP_PinActor_C" (Math|Transform|ComposeTransforms (.LocalTransform (Utilities|Struct|BreakS_PinSpawn _array_element)) (Transformation|GetActorTransform)) "Undefined" "MultiplyWithRoot" 0 (.PinDef (Utilities|Struct|BreakS_PinSpawn _array_element)) 0))
        (bind _output_get (LocalVariables|SetLoopPinSpawned _returnvalue))
        (Default|InitializePin _output_get)
        (Utilities|Array|Add (Variables|Default|GetSpawnedPins) (LocalVariables|GetLoopPinSpawned))))
    (:Is%20Not%20Valid
      (Development|PrintString "Invalid Layout"))))

(fn ClearExistingPins
  (bind _spawnedpins (Variables|Default|GetSpawnedPins))
  (for _array_element _spawnedpins
    (Utilities|IsValid _array_element
      (:Is%20Valid
        (Actor|DestroyActor _array_element))))
  (Utilities|Array|Clear _spawnedpins))

(fn GetKnockedPinCount
  (for _array_element (Variables|Default|GetSpawnedPins)
    (Utilities|IsValid _array_element
      (:Is%20Valid
        (bind _knockeddown (Default|IsKnockedDown _array_element))
        (if _knockeddown
          (Math|Integer|IncrementInt (LocalVariables|GetLoopCount))))))
  (return (LocalVariables|GetLoopCount)))

(fn RemoveKnockedDownPins
  (for _array_element (Variables|Default|GetSpawnedPins)
    (if (Variables|/Game/Core/Pins/BP_PinActor.BP_PinActor_C|GetbCountAsKnocked _array_element)
      (Utilities|Array|Add (LocalVariables|GetPinsToRemove) _array_element)))
  (for _array_element_2 (LocalVariables|GetPinsToRemove)
    (Actor|DestroyActor _array_element_2)))

(fn GetNewlyKnockedStandardPinCount
  (for _array_element (Variables|Default|GetSpawnedPins)
    (Utilities|IsValid _array_element
      (:Is%20Valid
        (bind _output_get (LocalVariables|SetLoopPin _array_element))
        (bind _knockeddown (Default|IsKnockedDown _output_get))
        (if (Math|Boolean|ANDBoolean _knockeddown (== (Variables|/Game/Core/Pins/BP_PinActor.BP_PinActor_C|GetbCountAsKnocked _output_get) false) (Variables|/Game/Data/Pins/PDA_PinDef.PDA_PinDef_C|GetbContributesToStandardBowlingRules (Variables|/Game/Core/Pins/BP_PinActor.BP_PinActor_C|GetPinDef _output_get)))
          (Math|Integer|IncrementInt (LocalVariables|GetLoopCount))))))
  (return (LocalVariables|GetLoopCount)))

(fn GetNewlyKnockedPinCount
  (for _array_element (Variables|Default|GetSpawnedPins)
    (Utilities|IsValid _array_element
      (:Is%20Valid
        (bind _output_get (LocalVariables|SetLoopPin _array_element))
        (bind _knockeddown (Default|IsKnockedDown _output_get))
        (if (and _knockeddown (== (Variables|/Game/Core/Pins/BP_PinActor.BP_PinActor_C|GetbCountAsKnocked _output_get) false))
          (Math|Integer|IncrementInt (LocalVariables|GetLoopCount)
            (:%20%20
              (Variables|/Game/Core/Pins/BP_PinActor.BP_PinActor_C|SetbCountAsKnocked (LocalVariables|GetLoopPin) true) ; If it's the first time we're counting them, don't count them in the future.
            ))))))
  (return (LocalVariables|GetLoopCount)))

(fn GetTotalPinCount
  (return (Utilities|Array|Length (Variables|Default|GetSpawnedPins))))

(fn GetStandardPinCount
  (params (CountStanding :type Boolean) (CountFallen :type Boolean))
  (for _array_element (Variables|Default|GetSpawnedPins)
    (Utilities|IsValid _array_element
      (:Is%20Valid
        (bind _output_get (LocalVariables|SetLoop_PinToCheck _array_element))
        (if (Variables|/Game/Data/Pins/PDA_PinDef.PDA_PinDef_C|GetbContributesToStandardBowlingRules (Variables|/Game/Core/Pins/BP_PinActor.BP_PinActor_C|GetPinDef _output_get))
          (if (and CountStanding CountFallen)
            (Math|Integer|IncrementInt (LocalVariables|GetLoopCount) :!label _label)
            (else
              (Utilities|FlowControl|Sequence
                (:then_0
                  (if (and CountStanding (not (Variables|/Game/Core/Pins/BP_PinActor.BP_PinActor_C|GetbCountAsKnocked (LocalVariables|GetLoop_PinToCheck))))
                    (goto _label)))
                (:then_1
                  (if (and CountFallen (Variables|/Game/Core/Pins/BP_PinActor.BP_PinActor_C|GetbCountAsKnocked (LocalVariables|GetLoop_PinToCheck)))
                    (goto _label))))))))))
  (return (LocalVariables|GetLoopCount)))
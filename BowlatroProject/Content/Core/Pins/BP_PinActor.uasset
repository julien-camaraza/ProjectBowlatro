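; BP_PinActor is a pin actor that can report whether it has been knocked down.
; InitializePin applies the mesh, material and mass override from its PinDef to PinMesh and clears KnockedDown, printing a message if PinDef is invalid.
; IsKnockedDown compares the mesh's up vector to world up with a dot product, flagging the pin as down once it tilts past a threshold.
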(event Custom|InitializePin
  (Utilities|IsValid (Variables|Default|GetPinDef)
    (:Is%20Valid
      (Components|StaticMesh|SetStaticMesh (Variables|Default|GetPinMesh) (Variables|/Game/Data/Pins/PDA_PinDef.PDA_PinDef_C|GetMesh (Variables|Default|GetPinDef)))
      (Rendering|Material|SetMaterial (Variables|Default|GetPinMesh) 0 (Variables|/Game/Data/Pins/PDA_PinDef.PDA_PinDef_C|GetMaterial (Variables|Default|GetPinDef)))
      (Class|PrimitiveComponent|SetMassOverrideinKg (Variables|Default|GetPinMesh) "None" (Variables|/Game/Data/Pins/PDA_PinDef.PDA_PinDef_C|GetMassKG (Variables|Default|GetPinDef)) true)
      (Variables|Default|SetbKnockedDown false))
    (:Is%20Not%20Valid
      (Development|PrintString "Pin Def is invalid"))))

(event EventBeginPlay)

(event Collision|EventActorBeginOverlap
  (params (OtherActor :type Actor%20Object%20Reference)))

(event EventTick
  (params (DeltaSeconds :type Float%20%28single-precision%29)))

(fn ConstructionScript)

(fn IsKnockedDown
  (bind _output_get (Variables|Default|SetbKnockedDown (< (Math|Vector|DotProduct (Math|Vector|GetUpVector (Variables|Default|GetPinMesh)) "0.000000,0.000000,1.000000") 0.8)))
  (return _output_get))
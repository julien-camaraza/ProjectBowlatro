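; Run manager for a bowling roguelike, tracking round progression, gold reward values and shop offers.
; StartRun expands RunStructureDef's stage tunings into three rounds per stage, the last a boss, which AdvanceRound steps through by index.
; The debug shop builds rarity-priced offers around a placeholder perk asset.
; Purchases charge PlayerState currency and mark offers sold, but only perks are granted; other types still cost gold.
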(event EventBeginPlay)

(event Collision|EventActorBeginOverlap
  (params (OtherActor :type Actor%20Object%20Reference)))

(event EventTick
  (params (DeltaSeconds :type Float%20%28single-precision%29)))

(fn ConstructionScript)

(fn StartRun
  (bind _currentround (GettersandSetters|GetCurrentRound))
  (bind (_requiredscore _displayname) (Utilities|Struct|BreakS_RunRoundDef _currentround))
  (BaseFlow|GenerateRunRounds)
  (Variables|Level|SetCurrentStageIndex 0)
  (Variables|Level|SetCurrentLevel (Utilities|Array|Get(acopy) (Variables|Level|GetLevelSequence)))
  (Variables|StageStructure|SetCurrentRoundIndex 0)
  (Development|PrintString (Utilities|String|ToString(Text) (Utilities|Text|FormatText "Generated rounds: {0} 
Current Round: {1} 
Required Score: {2}" (Utilities|Array|Length (Variables|StageStructure|GetGeneratedRounds)) _displayname _requiredscore))))

(fn GetCurrentLevel
  (return (Variables|Level|GetCurrentLevel)))

(fn AdvanceLevel)

(fn AddGold
  (params (Amount :type Integer))
  (bind _output_get (Variables|PlayerVars|SetGold (+ Amount (Variables|PlayerVars|GetGold))))
  (return _output_get))

(fn GenerateDebugShop
  (Utilities|Array|Clear (Variables|Shop|GetCurrentShopOffers))
  (for _array_element (Variables|Debug|GetDebugShopOffers)
    (Utilities|Array|Add (Variables|Shop|GetCurrentShopOffers) (Utilities|Struct|MakeS_ShopOffer "NewEnumerator3" "/Game/Data/Perks/DA_Perk_TestCommon.DA_Perk_TestCommon" (Variables|/Game/Data/Perks/PDA_PerkDef.PDA_PerkDef_C|GetDisplayName _array_element) (Variables|/Game/Data/Perks/PDA_PerkDef.PDA_PerkDef_C|GetDescription _array_element) (Utilities|Select :Index (Variables|/Game/Data/Perks/PDA_PerkDef.PDA_PerkDef_C|GetRarity _array_element) :NewEnumerator0 5 :NewEnumerator1 8 :NewEnumerator2 10 :NewEnumerator3 20) (Variables|/Game/Data/Perks/PDA_PerkDef.PDA_PerkDef_C|GetRarity _array_element)))))

(fn TryPurchaseShopOffer
  (params (ShopIndex :type Integer) (PlayerState :type BP%20Bowlatro%20Player%20State%20Object%20Reference))
  ;[0.15 0.15 0.15 0.5] Is valid
  (if (Utilities|Array|IsValidIndex (Variables|Shop|GetCurrentShopOffers) ShopIndex)
    (LocalVariables|SetIndexedShopOffer (Utilities|Array|Get(acopy) (Variables|Shop|GetCurrentShopOffers) ShopIndex))
    (LocalVariables|SetObjectPrice (Utilities|Struct|BreakS_ShopOffer (LocalVariables|GetIndexedShopOffer)))
    ;[0.15 0.15 0.15 0.5] Already purchased
    (if (Utilities|Struct|BreakS_ShopOffer (LocalVariables|GetIndexedShopOffer))
      (return false)
      (else
        ;[0.15 0.15 0.15 0.5] Check we have enough gold. If so, drain it.
        (if (Default|CanAfford (Variables|/Game/Core/Framework/BP_BowlatroPlayerState.BP_BowlatroPlayerState_C|GetBPC_Currency PlayerState) (LocalVariables|GetObjectPrice))
          (Default|SpendGold (Variables|/Game/Core/Framework/BP_BowlatroPlayerState.BP_BowlatroPlayerState_C|GetBPC_Currency PlayerState) (LocalVariables|GetObjectPrice) "NewEnumerator5")
          ;[0.15 0.15 0.15 0.5] Mark as purchased
          (Utilities|Array|SetArrayElem (Variables|Shop|GetCurrentShopOffers) ShopIndex (Utilities|Struct|MakeS_ShopOffer (.ItemType (Utilities|Struct|BreakS_ShopOffer (LocalVariables|GetIndexedShopOffer))) (.OfferedAsset (Utilities|Struct|BreakS_ShopOffer (LocalVariables|GetIndexedShopOffer))) (.DisplayName (Utilities|Struct|BreakS_ShopOffer (LocalVariables|GetIndexedShopOffer))) (.Description (Utilities|Struct|BreakS_ShopOffer (LocalVariables|GetIndexedShopOffer))) (.Price (Utilities|Struct|BreakS_ShopOffer (LocalVariables|GetIndexedShopOffer))) (.Rarity (Utilities|Struct|BreakS_ShopOffer (LocalVariables|GetIndexedShopOffer))) true))
          (switch Utilities|FlowControl|Switch|SwitchonE_ShopItemType (Utilities|Struct|BreakS_ShopOffer (LocalVariables|GetIndexedShopOffer)) ; Maybe add an "On Purchase" event here
            (:NewEnumerator0
              _)
            (:NewEnumerator1
              _)
            (:NewEnumerator2
              _)
            (:NewEnumerator3
              (Default|AddPerk (Variables|/Game/Core/Framework/BP_BowlatroPlayerState.BP_BowlatroPlayerState_C|GetBPC_PerkInventory PlayerState) (.AsPDA%20Perk%20Def (Utilities|Casting|CastToPDA_PerkDef (Utilities|Struct|BreakS_ShopOffer (LocalVariables|GetIndexedShopOffer)))))
              (return true)))
          (Development|PrintString "Upgrade type not purchasable yet!" true true "(R=1.000000,G=0.018067,B=0.000000,A=1.000000)" 4.0)
          (return false)
          (else
            (Development|PrintString "Too poor!" true true "(R=1.000000,G=0.018067,B=0.000000,A=1.000000)" 4.0)
            (return false)))))
    (else
      (return false))))

(fn GetGoldPerRemainingFrame
  (return (Variables|PlayerVars|GetBaseGoldPerRemainingFrame)))

(fn GetGoldGainPerLevel
  (return (Variables|PlayerVars|GetBaseGoldGainPerRound)))

(fn GenerateRunRounds
  (Utilities|Array|Clear (Variables|StageStructure|GetGeneratedRounds))
  (Utilities|IsValid (Variables|StageStructure|GetRunStructureDef)
    (:Is%20Valid
      (for (_array_element _array_index) (Variables|/Game/Data/Levels/PDA_RunStructureDef.PDA_RunStructureDef_C|GetStageTunings (Variables|StageStructure|GetRunStructureDef))
        (LocalVariables|SetLoop_StageTuning _array_element)
        (LocalVariables|SetLoop_ArrayIndexAdjusted (+ _array_index 1))
        (Utilities|FlowControl|Sequence ; Each round is a line on the sequence for now.
          (:then_0
            ;[0.15 0.15 0.15 0.5] Round 1
            (Utilities|Array|Add (Variables|StageStructure|GetGeneratedRounds) (Utilities|Struct|MakeS_RunRoundDef (LocalVariables|GetLoop_ArrayIndexAdjusted) 1 (.BaseRequiredScore (Utilities|Struct|BreakS_StageTuning (LocalVariables|GetLoop_StageTuning))) (.FrameCount (Utilities|Struct|BreakS_StageTuning (LocalVariables|GetLoop_StageTuning))) "/Game/Data/PinLayouts/DA_PinLayout_Standard10.DA_PinLayout_Standard10" false 0 0 (Utilities|Text|FormatText "Level:{0}-1" (LocalVariables|GetLoop_ArrayIndexAdjusted)))))
          (:then_1
            ;[0.15 0.15 0.15 0.5] Round 2
            (Utilities|Array|Add (Variables|StageStructure|GetGeneratedRounds) (Utilities|Struct|MakeS_RunRoundDef (LocalVariables|GetLoop_ArrayIndexAdjusted) 2 (Math|Float|Round (* (.BaseRequiredScore (Utilities|Struct|BreakS_StageTuning (LocalVariables|GetLoop_StageTuning))) (Variables|/Game/Data/Levels/PDA_RunStructureDef.PDA_RunStructureDef_C|GetRound2ScoreMultiplier (Variables|StageStructure|GetRunStructureDef)))) (.FrameCount (Utilities|Struct|BreakS_StageTuning (LocalVariables|GetLoop_StageTuning))) "/Game/Data/PinLayouts/DA_PinLayout_Standard10.DA_PinLayout_Standard10" false 0 0 (Utilities|Text|FormatText "Level:{0}-2" (LocalVariables|GetLoop_ArrayIndexAdjusted)))))
          (:then_2
            ;[0.15 0.15 0.15 0.5] Round 3 (Boss)
            (Utilities|Array|Add (Variables|StageStructure|GetGeneratedRounds) (Utilities|Struct|MakeS_RunRoundDef (LocalVariables|GetLoop_ArrayIndexAdjusted) 3 (Math|Float|Round (* (.BaseRequiredScore (Utilities|Struct|BreakS_StageTuning (LocalVariables|GetLoop_StageTuning))) 1.0)) (.FrameCount (Utilities|Struct|BreakS_StageTuning (LocalVariables|GetLoop_StageTuning))) "/Game/Data/PinLayouts/DA_PinLayout_Standard10.DA_PinLayout_Standard10" true 0 0 (Utilities|Text|FormatText "Level:{0}-Boss" (LocalVariables|GetLoop_ArrayIndexAdjusted))))))))
    (:Is%20Not%20Valid
      (Development|PrintString "Missing RunStructureDef"))))

(fn GetCurrentRound
  (return (Utilities|Array|Get(acopy) (Variables|StageStructure|GetGeneratedRounds) (Variables|StageStructure|GetCurrentRoundIndex))))

(fn AdvanceRound
  (Math|Integer|IncrementInt (Variables|StageStructure|GetCurrentRoundIndex)))
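; BP_BowlingBallActor is the physics bowling ball actor, configured from a ball instance and its definition.
; InitializeBall applies mesh, material, mass and base score with permanent bonus, but scales the actor by throw-speed multiplier rather than stored size scale.
; ThrowBall impulses along mesh forward using strength and multiplier, ignoring ThrowDirection and adding zeroed torque.
; Spin values are stored, but HandleSpin is empty and its sideways-force logic is disconnected.
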(event EventBeginPlay)

(event Collision|EventActorBeginOverlap
  (params (OtherActor :type Actor%20Object%20Reference)))

(event EventTick
  (params (DeltaSeconds :type Float%20%28single-precision%29)))

(fn ConstructionScript)

(fn InitializeBall
  (params (BallInstance :type S%20Ball%20Instance%20Structure%20%28by%20ref%29))
  (bind _output_get (Variables|Default|SetBallInstance BallInstance))
  (Utilities|IsValid (.BallDef (Utilities|Struct|BreakS_BallInstance _output_get))
    (:Is%20Valid
      (Variables|Default|SetBallDef (.BallDef (Utilities|Struct|BreakS_BallInstance _output_get)))
      (Components|StaticMesh|SetStaticMesh (Variables|Default|GetBallMesh) (Variables|/Game/Data/PDA_BallDef.PDA_BallDef_C|GetBallMesh (Variables|Default|GetBallDef)))
      (Rendering|Material|SetMaterial (Variables|Default|GetBallMesh) 0 (Variables|/Game/Data/PDA_BallDef.PDA_BallDef_C|GetBallMaterial (Variables|Default|GetBallDef)))
      (Variables|Default|SetFinalBaseScore (+ (Variables|/Game/Data/PDA_BallDef.PDA_BallDef_C|GetBaseScore (Variables|Default|GetBallDef)) (.PermanentBaseScoreBonus (Utilities|Struct|BreakS_BallInstance (Variables|Default|GetBallInstance)))))
      (bind _output_get_2 (Variables|Default|SetFinalWeightLlbs (Variables|/Game/Data/PDA_BallDef.PDA_BallDef_C|GetWeightLbs (Variables|Default|GetBallDef))))
      (Variables|Default|SetFinalWeightKg (* _output_get_2 0.453592))
      (Class|PrimitiveComponent|SetMassOverrideinKg (Variables|Default|GetBallMesh) "None" (Variables|Default|GetFinalWeightKg) true)
      (Variables|Default|SetFinalSizeScale (Variables|/Game/Data/PDA_BallDef.PDA_BallDef_C|GetSizeScale (Variables|Default|GetBallDef)))
      (bind _output_get_3 (Variables|Default|SetFinalThrowSpeedMultiplier (Variables|/Game/Data/PDA_BallDef.PDA_BallDef_C|GetThrowSpeedMult (Variables|Default|GetBallDef))))
      (Transformation|SetActorScale3D (Math|Vector|MakeVector _output_get_3 _output_get_3 _output_get_3)))
    (:Is%20Not%20Valid
      (Development|PrintString "Invalid ball def"))))

(fn ThrowBall
  (params (ThrowDirection :type Vector) (ThrowStrength :type Float%20%28double-precision%29))
  (bind _output_get (LocalVariables|SetFinalImpulse (* (Math|Vector|GetForwardVector (Variables|Default|GetBallMesh)) (* ThrowStrength 1e+01) (Variables|Default|GetFinalThrowSpeedMultiplier))))
  (Class|PrimitiveComponent|AddTorqueinDegrees (Variables|Default|GetBallMesh) (Math|Transform|TransformDirection (Transformation|GetWorldTransform (Variables|Default|GetBallMesh)) (* (Math|Vector|Normalize (Math|Vector|RotateVectorAroundAxis "0.000000,1.000000,0.000000" 9e+01 "1.000000,1.000000,0.000000")) "0.000000,0.000000,0.000000")) "None" false)
  (Physics|AddImpulse (Variables|Default|GetBallMesh) _output_get "None" false))

(fn SetSpin
  (params (NewSpinAmount :type Float%20%28double-precision%29) (NewSpinForce :type Float%20%28double-precision%29))
  (Variables|Default|SetSpinAmount NewSpinAmount)
  (Variables|Default|SetSpinForce NewSpinForce))

(fn HandleSpin)

(fn EndThrow
  (Variables|Default|SetbApplySpin false))
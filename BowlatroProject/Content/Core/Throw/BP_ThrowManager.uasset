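; Throw manager for a bowling-style game that detects when a throw has come to rest and notifies the LaneManager.
; BeginThrow registers the ball as the active one.
; During one LaneManager run phase, Tick polls ball and pin physics velocities against separate movement thresholds.
; Once everything stays below them for a continuous settle time, FinishThrow resets its state and calls HandleThrowFinished; any movement restarts the timer.
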(event EventBeginPlay)

(event Collision|EventActorBeginOverlap
  (params (OtherActor :type Actor%20Object%20Reference)))

(event EventTick
  (params (DeltaSeconds :type Float%20%28single-precision%29))
  (if (Utilities|Enum|Equal(Enum) (Variables|/Game/Core/Lane/BP_LaneManager.BP_LaneManager_C|GetCurrentRunPhase (Variables|References|GetLaneManager)) "NewEnumerator5")
    (bind _finished (CallFunction|CheckThrowFinished))
    (if _finished
      (bind _output_get (Variables|Trackers|SetCurrentSettleTime (+ (Variables|Trackers|GetCurrentSettleTime) (Utilities|Time|GetWorldDeltaSeconds))))
      (if (>= _output_get (Variables|Controllers|GetSettleTimeRequired))
        (CallFunction|FinishThrow))
      (else
        (Variables|Trackers|SetCurrentSettleTime 0.0)))))

(fn ConstructionScript)

(fn BeginThrow
  (params (BallActor :type BP%20Bowling%20Ball%20Actor%20Object%20Reference))
  (bind _activeballactors (Variables|Trackers|GetActiveBallActors))
  (Utilities|Array|Clear _activeballactors)
  (Utilities|Array|Add _activeballactors BallActor)
  (Variables|Trackers|SetThrowInProgress true))

(fn CheckThrowFinished
  (bind _lanemanager (Variables|References|GetLaneManager))
  (bind _pinrack (Variables|/Game/Core/Lane/BP_LaneManager.BP_LaneManager_C|GetPinRack _lanemanager))
  ;[0.15 0.15 0.15 0.5] Check if any ball has a velocity with a vector length of 5 or more. As soon as we hit, consider it a failure. Otherwise pass.
  (for _array_element (Variables|Trackers|GetActiveBallActors)
    (bind _returnvalue (Physics|GetPhysicsLinearVelocity (Variables|/Game/Core/Balls/BP_BowlingBallActor.BP_BowlingBallActor_C|GetBallMesh _array_element) "None"))
    (if (> (Math|Vector|VectorLength _returnvalue) (Variables|Controllers|GetBallMinimumVelocityToBeConsideredMoving))
      (return false)))
  ;[0.15 0.15 0.15 0.5] Now check if any of the pins are moving
  (Utilities|IsValid _pinrack
    (:Is%20Valid
      (for _array_element_2 (Variables|/Game/Core/Pins/BP_PinRack.BP_PinRack_C|GetSpawnedPins _pinrack)
        (Utilities|IsValid (Variables|/Game/Core/Pins/BP_PinActor.BP_PinActor_C|GetPinMesh _array_element_2)
          (:Is%20Valid
            (bind _returnvalue_2 (Physics|GetPhysicsLinearVelocity (Variables|/Game/Core/Pins/BP_PinActor.BP_PinActor_C|GetPinMesh _array_element_2) "None"))
            (if (> (Math|Vector|VectorLength _returnvalue_2) (Variables|Controllers|GetPinMinimumVelocityToBeConsideredMoving))
              (return false)))))
      (return true))))

(fn FinishThrow
  (Variables|Trackers|SetThrowInProgress false)
  (Variables|Trackers|SetCurrentSettleTime 0.0)
  (bind _lanemanager (Variables|References|GetLaneManager)
    (:then
      (Default|HandleThrowFinished _lanemanager))
    (:else)))
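; Bowling aim and throw manager that spawns the selected ball and handles its positioning, aim, spin and power until release.
; LaneManager run phases gate most inputs; positioning and aiming briefly toggle physics to move or rotate the ball, with a debug aim line.
; Tick ping-pongs the power meter while charging.
; Release sends LaneManager a direction from the aim angle, separate from the aim-line target, and power-scaled strength.
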(event EventBeginPlay
  (bind _outactors (Actor|GetAllActorsOfClass "/Game/Core/Lane/BP_LaneManager.BP_LaneManager_C"))
  (Variables|Default|SetLaneManager (Utilities|Array|Get(acopy) _outactors)))

(event EventTick
  (params (DeltaSeconds :type Float%20%28single-precision%29))
  (Variables|Internal|SetDeltaSeconds DeltaSeconds)
  (AimingandThrowing|HandlePowerMeter)
  (if (Utilities|Enum|Equal(Enum) (Variables|/Game/Core/Lane/BP_LaneManager.BP_LaneManager_C|GetCurrentRunPhase (Variables|Default|GetLaneManager)) "NewEnumerator4")
    (Rendering|Debug|DrawDebugLine (Transformation|GetWorldLocation (Variables|/Game/Core/Balls/BP_BowlingBallActor.BP_BowlingBallActor_C|GetBallMesh (Variables|References|GetActiveBallActor))) (Variables|Throwing|GetBallAimLocation) "(R=0.397363,G=1.000000,B=0.737453,A=1.000000)" 0.0 2.0)))

(fn ConstructionScript)

(fn SelectBallforThrow
  (params (BallInstance :type S%20Ball%20Instance%20Structure))
  (bind _output_get (Variables|ThrowTracking|SetCurrentBallInstance BallInstance))
  (bind _returnvalue (Game|SpawnActorfromClass (Variables|BowlingBall|GetBallActorClass) (Variables|BowlingBall|GetBowlingBallTransform) "Undefined" "MultiplyWithRoot" 0 (.BallDef (Utilities|Struct|BreakS_BallInstance _output_get)) 0))
  (bind _output_get_2 (Variables|References|SetActiveBallActor _returnvalue))
  (Default|InitializeBall _output_get_2 BallInstance)
  (Default|EnterRunPhase (Variables|Default|GetLaneManager) "NewEnumerator4")
  (Variables|Throwing|SetSpinAmount 0.0)
  (Variables|Throwing|SetPowerAmount (Variables|Throwing|GetMinPower))
  (Variables|Internal|SetPowerCharingDirection 1.0)
  (Variables|Throwing|SetAimAngleDegrees 0.0)
  (Variables|Throwing|SetbAimingActive true))

(fn SetAimAngle
  (params (NewAimAngle :type Float%20%28double-precision%29))
  (bind _maxaimangledegrees (Variables|Controllers|GetMaxAimAngleDegrees))
  (if (Utilities|Enum|Equal(Enum) (Variables|Internal|GetCurrentRunPhase) "NewEnumerator4")
    (Variables|Throwing|SetAimAngleDegrees (Math|Float|Clamp(Float) NewAimAngle (* _maxaimangledegrees -1.0) _maxaimangledegrees))))

(fn GetCurrentThrowDirection
  (return (Math|Vector|Normalize (Math|Vector|RotateVectorAroundAxis (Math|Vector|MakeVector 1.0 0.0 0.0) (Variables|Throwing|GetAimAngleDegrees) "0.000000,0.000000,1.000000"))))

(fn SetSpinAmount
  (params (NewSpinAmount :type Float%20%28double-precision%29))
  (if (Utilities|Enum|Equal(Enum) (Variables|Internal|GetCurrentRunPhase) "NewEnumerator4")
    (Variables|Throwing|SetSpinAmount (Math|Float|Clamp(Float) NewSpinAmount (* -1.0 (Variables|Controllers|GetMaxSpinAmount)) (Variables|Controllers|GetMaxSpinAmount)))))

(fn SetPowerAmount
  (params (NewPowerAmount :type Float%20%28double-precision%29))
  (Variables|Throwing|SetPowerAmount (Math|Float|Clamp(Float) NewPowerAmount (Variables|Throwing|GetMinPower) (Variables|Throwing|GetMaxPower))))

(fn StartChargingPower
  (if (Utilities|Enum|Equal(Enum) (Variables|/Game/Core/Lane/BP_LaneManager.BP_LaneManager_C|GetCurrentRunPhase (Variables|Default|GetLaneManager)) "NewEnumerator4")
    (Default|EnterRunPhase (Variables|Default|GetLaneManager) "NewEnumerator11")
    (Variables|Throwing|SetbChargingPower true)
    (Variables|Throwing|SetPowerAmount (Variables|Throwing|GetMinPower))
    (Variables|Internal|SetPowerCharingDirection 1.0)))

(fn ReleasePowerandThrow
  (Variables|Throwing|SetbAimingActive false)
  (Variables|Throwing|SetbChargingPower false)
  (Default|RequestBallThrow (Variables|Default|GetLaneManager) (AimingandThrowing|GetCurrentThrowDirection) (* (Variables|Controllers|GetThrowStrength) (Variables|Throwing|GetPowerAmount)) (Variables|References|GetActiveBallActor)))

(fn HandlePowerMeter
  (if (Variables|Throwing|GetbChargingPower)
    (LocalVariables|SetNewPower (+ (* (Variables|Internal|GetDeltaSeconds) (Variables|Throwing|GetPowerChargeSpeed) (Variables|Internal|GetPowerCharingDirection)) (Variables|Throwing|GetPowerAmount)))
    (Utilities|FlowControl|Sequence
      (:then_0
        ;[0.15 0.15 0.15 0.5] Ping pong the meter
        (if (>= (LocalVariables|GetNewPower) (Variables|Throwing|GetMaxPower))
          (Variables|Internal|SetPowerCharingDirection -1.0)
          (elif (<= (LocalVariables|GetNewPower) (Variables|Throwing|GetMinPower))
            (Variables|Internal|SetPowerCharingDirection 1.0))))
      (:then_1
        (Variables|Throwing|SetPowerAmount (LocalVariables|GetNewPower))))))

(fn AimBall
  (params (ActionValue :type Vector%202D%20Structure))
  (bind _activeballactor (Variables|References|GetActiveBallActor))
  (bind _ballmesh (Variables|/Game/Core/Balls/BP_BowlingBallActor.BP_BowlingBallActor_C|GetBallMesh _activeballactor))
  (if (Utilities|Enum|Equal(Enum) (Variables|/Game/Core/Lane/BP_LaneManager.BP_LaneManager_C|GetCurrentRunPhase (Variables|Default|GetLaneManager)) "NewEnumerator4")
    (Variables|Throwing|SetBallAimLocation (Math|Vector|MakeVector (.x (Variables|Throwing|GetBallAimLocation)) (+ (.y (Variables|Throwing|GetBallAimLocation)) (* (.x ActionValue) 2.0)) (.z (Variables|Throwing|GetBallAimLocation))))
    (Variables|Throwing|SetbAimingActive true)
    (Physics|SetSimulatePhysics _ballmesh false)
    (Transformation|SetWorldRotation _ballmesh (Math|Rotator|FindLookatRotation (Transformation|GetWorldLocation _ballmesh) (Variables|Throwing|GetBallAimLocation)) false false)
    (Physics|SetSimulatePhysics _ballmesh true)))

(fn MoveStartingBallLocation
  (params (ActionValue :type Vector%202D%20Structure))
  (bind _activeballactor (Variables|References|GetActiveBallActor))
  (bind _ballmesh (Variables|/Game/Core/Balls/BP_BowlingBallActor.BP_BowlingBallActor_C|GetBallMesh _activeballactor))
  (bind _ballmesh_2 (Variables|/Game/Core/Balls/BP_BowlingBallActor.BP_BowlingBallActor_C|GetBallMesh _activeballactor))
  (bind _returnvalue (Transformation|GetWorldLocation _ballmesh_2))
  (if (Utilities|Enum|Equal(Enum) (Variables|/Game/Core/Lane/BP_LaneManager.BP_LaneManager_C|GetCurrentRunPhase (Variables|Default|GetLaneManager)) "NewEnumerator4")
    (Physics|SetSimulatePhysics _ballmesh false)
    (Transformation|SetWorldLocation _ballmesh (Math|Vector|MakeVector (.x _returnvalue) (Math|Float|Min(Float) (Math|Float|Max(Float) (+ (.x ActionValue) (.y _returnvalue)) -51.0) 51.0) (.z _returnvalue)) false true)
    (Physics|SetSimulatePhysics _ballmesh true)))
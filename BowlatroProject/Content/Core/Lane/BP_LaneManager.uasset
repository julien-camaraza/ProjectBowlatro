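; Lane manager for a bowling game that runs a level from pin setup through frames, throws and scoring to win or fail.
; A run-phase enum gates ball choice, aim, spin and a ping-pong power meter before the throw.
; Finished throws become a result struct passed through score resolver and effect router components.
; After the controller's scoring ceremony, the score and throw count decide level end, next frame or next throw.
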(event EventBeginPlay
  (Initialize|InitializeSecondaryActors))

(event EventTick
  (params (DeltaSeconds :type Float%20%28single-precision%29))
  (Variables|Internal|SetDeltaSeconds DeltaSeconds)
  (AimingandThrowing|HandlePowerMeter)
  (if (Variables|Throwing|GetbAimingActive)
    (Rendering|Debug|DrawDebugLine (Transformation|GetWorldLocation (Variables|/Game/Core/Balls/BP_BowlingBallActor.BP_BowlingBallActor_C|GetBallMesh (Variables|References|GetActiveBallActor))) (Variables|Throwing|GetBallAimLocation) "(R=0.397363,G=1.000000,B=0.737453,A=1.000000)" 0.0 2.0)))

(fn ConstructionScript)

(fn EnterRunPhase
  (params (CurrentRunPhase :type E_RunPhase%20Enum :default "NewEnumerator0"))
  ;[0.15 0.15 0.15 0.5] Easy function in case we want more here. Currently the same as just changing the variable
  (Variables|Internal|SetCurrentRunPhase CurrentRunPhase))

(fn StartLevel
  (params (LevelToStart :type PDA%20Level%20Def%20Object%20Reference))
  (Utilities|IsValid LevelToStart
    (:Is%20Valid
      (Initialize|ClearLane)
      (LevelFlow|EnterRunPhase "NewEnumerator2")
      (Variables|References|SetActiveLevelDef LevelToStart)
      (Default|MarkAllBallsUnused (Variables|/Game/Core/Framework/BP_BowlatroPlayerState.BP_BowlatroPlayerState_C|GetBPC_BallInventory (Variables|References|GetActivePlayerState)))
      ;[0.15 0.15 0.15 0.5] Reset vars for level and set up pins
      (Variables|CurrentLevelTrackers|SetCurrentLevelScore 0)
      (Variables|CurrentLevelTrackers|SetThrowsUsed 0)
      (Variables|CurrentLevelTrackers|SetThrowsPerFrame (Variables|/Game/Data/Levels/PDA_LevelDef.PDA_LevelDef_C|GetThrowsPerFrame LevelToStart))
      (Variables|CurrentLevelTrackers|SetFrameCount (Variables|/Game/Data/Levels/PDA_LevelDef.PDA_LevelDef_C|GetFrames LevelToStart))
      (Variables|CurrentLevelTrackers|SetTargetScore (Variables|/Game/Data/Levels/PDA_LevelDef.PDA_LevelDef_C|GetTargetScore LevelToStart))
      (Utilities|IsValid (Variables|References|GetPinRack)
        (:Is%20Valid
          (LevelFlow|StartFrame))
        (:Is%20Not%20Valid
          (Development|PrintString "Lane Manager has an invalid pin rack" true true "(R=1.000000,G=0.000000,B=0.054410,A=1.000000)" 1e+01))))
    (:Is%20Not%20Valid
      (Development|PrintString "Invalid Level Def" true true "(R=1.000000,G=0.061983,B=0.000000,A=1.000000)" 1e+01))))

(fn StartFrame
  (LevelFlow|EnterRunPhase "NewEnumerator12")
  (Variables|CurrentLevelTrackers|SetThrowIndexInFrame 0)
  (Default|SpawnPinsfromLayout (Variables|References|GetPinRack) (Variables|/Game/Data/Levels/PDA_LevelDef.PDA_LevelDef_C|GetPinLayout (Variables|References|GetActiveLevelDef)))
  (LevelFlow|TriggerBallChoosing))

(fn TriggerBallChoosing
  (LevelFlow|EnterRunPhase "NewEnumerator3")
  (bind _asbp_bowlatro_player_controller (Utilities|Casting|CastToBP_BowlatroPlayerController (Game|GetPlayerController (Variables|References|GetActivePlayerState))))
  (Default|StartChoosingBall _asbp_bowlatro_player_controller))

(fn SelectFirstAvailableBall
  (LevelFlow|EnterRunPhase "NewEnumerator3")
  (bind _output_get (VariableGetters|GetAvailableBallInstances))
  (if (> (Utilities|Array|Length _output_get) 0)
    (LevelFlow|SelectBallforThrow (Utilities|Array|Get(acopy) (LocalVariables|GetBallsAvailable)))
    (else
      (Development|PrintString "No balls left!" true true "(R=1.000000,G=0.000086,B=0.021884,A=1.000000)" 1e+01))))

(fn SelectBallforThrow
  (params (BallInstance :type S%20Ball%20Instance%20Structure))
  (bind _output_get (Variables|ThrowTracking|SetCurrentBallInstance BallInstance))
  (bind _returnvalue (Game|SpawnActorfromClass (Variables|BowlingBall|GetBallActorClass) (Variables|BowlingBall|GetBowlingBallTransform) "Undefined" "MultiplyWithRoot" 0 (.BallDef (Utilities|Struct|BreakS_BallInstance _output_get)) 0))
  (bind _output_get_2 (Variables|References|SetActiveBallActor _returnvalue))
  (Default|InitializeBall _output_get_2 BallInstance)
  (LevelFlow|EnterRunPhase "NewEnumerator4")
  (Variables|Throwing|SetSpinAmount 0.0)
  (Variables|Throwing|SetPowerAmount (Variables|Throwing|GetMinPower))
  (Variables|Internal|SetPowerCharingDirection 1.0)
  (Variables|Throwing|SetAimAngleDegrees 0.0))

(fn RequestBallThrow
  (params (Direction :type Vector) (Strength :type Float%20%28double-precision%29))
  ;[0.15 0.15 0.15 0.5] Throw ball
  (if (Utilities|Enum|Equal(Enum) (Variables|Internal|GetCurrentRunPhase) "NewEnumerator11")
    (Variables|References|GetActiveBallActor
      (:then
        (Default|BeginThrow (Variables|ThrowTracking|GetThrowManager) (Variables|References|GetActiveBallActor))
        (Utilities|FlowControl|Sequence
          (:then_1
            (Default|SetSpin (Variables|References|GetActiveBallActor) (Variables|Throwing|GetSpinAmount) (Variables|Throwing|GetSpinTurnForce))
            (Default|ThrowBall (Variables|References|GetActiveBallActor) Direction Strength)
            (LevelFlow|EnterRunPhase "NewEnumerator5")
            (return true))))
      (:else
        (Development|PrintString "Can't throw ball, no valid ball." true true "(R=1.000000,G=0.000000,B=0.013895,A=1.000000)" 1e+01)
        (return false)))
    (else
      (return false))))

(fn SpawnDebugBall)

(fn CheckifAllPinsWereKnockedDown
  (bind _pinrack (Variables|References|GetPinRack))
  (return (== (Default|GetKnockedPinCount _pinrack) (Utilities|Array|Length (Variables|/Game/Core/Pins/BP_PinRack.BP_PinRack_C|GetSpawnedPins _pinrack)))))

(fn InitializeSecondaryActors
  (bind _returnvalue (Game|GetPlayerController 0))
  (bind _playerstate (Variables|/Script/Engine.Controller|GetPlayerState _returnvalue))
  ;[0.15 0.15 0.15 0.5] Throw manager
  (Variables|References|SetBowlatroGameModeRef (.AsBP%20Bowlatro%20Game%20Mode (Utilities|Casting|CastToBP_BowlatroGameMode (Game|GetGameMode))))
  (bind _returnvalue_2 (Game|SpawnActorfromClass (Variables|ThrowTracking|GetThrowManagerClass) (Math|Transform|MakeTransform "0, 0, 0") "Undefined" "MultiplyWithRoot" 0 0))
  (bind _output_get (Variables|ThrowTracking|SetThrowManager _returnvalue_2))
  (Variables|/Game/Core/Throw/BP_ThrowManager.BP_ThrowManager_C|SetLaneManager _output_get self)
  (Utilities|IsValid _playerstate
    (:Is%20Valid
      (bind _asbp_bowlatro_player_state (Utilities|Casting|CastToBP_BowlatroPlayerState _playerstate))
      (Variables|References|SetActivePlayerState _asbp_bowlatro_player_state))
    (:Is%20Not%20Valid
      (Development|PrintString "No active player state" true true "(R=1.000000,G=0.007390,B=0.000000,A=1.000000)" 1e+01))))

(fn HandleThrowFinished
  (bind _pinrack (Variables|References|GetPinRack))
  (bind _pinrack_2 (Variables|References|GetPinRack))
  (bind _pinrack_3 (Variables|References|GetPinRack))
  (bind _pincount (Default|GetTotalPinCount _pinrack_2))
  (LevelFlow|EnterRunPhase "NewEnumerator6")
  (Default|EndThrow (Variables|References|GetActiveBallActor))
  (LocalVariables|SetNewlyKnockedStandardPinCount (Default|GetNewlyKnockedStandardPinCount (Variables|References|GetPinRack)))
  (LocalVariables|SetWasStrike (and (== (Default|GetStandardPinCount (Variables|References|GetPinRack) true true) (LocalVariables|GetNewlyKnockedStandardPinCount)) (== (Variables|ThrowTracking|GetCurrentThrowIndex) 0)))
  (bind _count (Default|GetNewlyKnockedPinCount (Variables|References|GetPinRack)))
  (LocalVariables|SetNewlyKnockedPinCount _count)
  ;[0.15 0.15 0.15 0.5] Set all data needed for last throw result
  (Variables|ThrowTracking|SetLastThrowResult (Utilities|Struct|MakeS_ThrowResult (Variables|ThrowTracking|GetCurrentBallInstance) (Variables|References|GetActiveBallActor) (Variables|References|GetActivePlayerState) (Variables|ThrowTracking|GetCurrentThrowIndex) (LocalVariables|GetNewlyKnockedPinCount) (LocalVariables|GetNewlyKnockedStandardPinCount) (Default|GetStandardPinCount _pinrack_3 true false) (Default|GetStandardPinCount _pinrack_3 false true) _pincount (- _pincount (Default|GetKnockedPinCount _pinrack_2)) (LevelFlow|CheckifAllPinsWereKnockedDown) (== (LocalVariables|GetNewlyKnockedPinCount) 0) (LocalVariables|GetWasStrike) (and (== (Default|GetStandardPinCount _pinrack true true) (Default|GetStandardPinCount _pinrack false true)) (not (LocalVariables|GetWasStrike)))))
  ;[0.15 0.15 0.15 0.5] Handle score
  (bind _scorecontext (Default|CalculateThrowScore (Variables|Default|GetBPC_ScoreResolver) (Variables|ThrowTracking|GetLastThrowResult)))
  (bind _modifiedscorecontext (Default|ApplyScoreEffects (Variables|Default|GetBPC_EffectRouter) _scorecontext (Variables|ThrowTracking|GetLastThrowResult) self))
  (bind _output_get (Variables|CurrentLevelTrackers|SetLastScoreContext _modifiedscorecontext))
  (Variables|CurrentLevelTrackers|SetCurrentLevelScore (+ (.FinalScore (Utilities|Struct|BreakS_ScoreContext _output_get)) (Variables|CurrentLevelTrackers|GetCurrentLevelScore)))
  ;[0.15 0.15 0.15 0.5] Tell inventory we used this ball
  (Default|MarkBallUsed (Variables|/Game/Core/Framework/BP_BowlatroPlayerState.BP_BowlatroPlayerState_C|GetBPC_BallInventory (Variables|References|GetActivePlayerState)) (.InstanceID (Utilities|Struct|BreakS_BallInstance (Variables|ThrowTracking|GetCurrentBallInstance))))
  ;[0.15 0.15 0.15 0.5] Handle internal trackers
  (Math|Integer|IncrementInt (Variables|ThrowTracking|GetCurrentThrowIndex)
    (:%20%20
      (Math|Integer|IncrementInt (Variables|CurrentLevelTrackers|GetThrowsUsed)
        (:%20%20
          (Math|Integer|IncrementInt (Variables|CurrentLevelTrackers|GetThrowIndexInFrame)
            (:%20%20
              (LevelFlow|StartScoringCeremony))))))))

(fn StartScoringCeremony
  (LevelFlow|EnterRunPhase "NewEnumerator6")
  (Default|ShowScoringCeremony (.AsBP%20Bowlatro%20Player%20Controller (Utilities|Casting|CastToBP_BowlatroPlayerController (Game|GetPlayerController (Variables|References|GetActivePlayerState))))))

(fn FinishScoringCeremony
  (LevelFlow|ResolveLevelState))

(fn ResolveLevelState
  (if (>= (Variables|CurrentLevelTrackers|GetCurrentLevelScore) (Variables|CurrentLevelTrackers|GetTargetScore))
    ;[0.15 0.15 0.15 0.5] Level Win. Gain Gold
    (LevelFlow|EnterRunPhase "NewEnumerator7")
    (Default|CallOnLevelCompleted)
    (Default|TriggerLevelEndGoldGain (Variables|References|GetBowlatroGameModeRef) (Variables|References|GetActivePlayerState) (Math|Integer|SelectInt (Utilities|Operators|Subtract (Variables|CurrentLevelTrackers|GetFrameCount) (Variables|CurrentLevelTrackers|GetCurrentFrameIndex) 1) (- (Variables|CurrentLevelTrackers|GetFrameCount) (Variables|CurrentLevelTrackers|GetCurrentFrameIndex)) (>= (+ (Variables|CurrentLevelTrackers|GetCurrentFrameIndex) 1) (Variables|CurrentLevelTrackers|GetThrowsPerFrame))))
    (elif (and (>= (+ (Variables|CurrentLevelTrackers|GetCurrentFrameIndex) 1) (Variables|CurrentLevelTrackers|GetFrameCount)) (>= (Variables|CurrentLevelTrackers|GetThrowIndexInFrame) (Variables|CurrentLevelTrackers|GetThrowsPerFrame)))
      (LevelFlow|EnterRunPhase "NewEnumerator10")
      (Default|CallOnLevelFailed)
      (Development|PrintString "No more throws")
      (elif (>= (Variables|CurrentLevelTrackers|GetThrowIndexInFrame) (Variables|CurrentLevelTrackers|GetThrowsPerFrame))
        (LevelFlow|EndFrame)
        (elif (Utilities|Struct|BreakS_ThrowResult (Variables|ThrowTracking|GetLastThrowResult))
          (LevelFlow|EndFrame)
          (else
            (LevelFlow|StartMidFrameThrow)))))))

(fn StartMidFrameThrow
  (Actor|DestroyActor (Variables|References|GetActiveBallActor))
  (Default|RemoveKnockedDownPins (Variables|References|GetPinRack))
  (LevelFlow|TriggerBallChoosing))

(fn EndFrame
  (Math|Integer|IncrementInt (Variables|CurrentLevelTrackers|GetCurrentFrameIndex)
    (:%20%20
      (LevelFlow|StartFrame))))

(fn SetAimAngle
  (params (NewAimAngle :type Float%20%28double-precision%29))
  (bind _maxaimangledegrees (Variables|Controllers|GetMaxAimAngleDegrees))
  (if (Utilities|Enum|Equal(Enum) (Variables|Internal|GetCurrentRunPhase) "NewEnumerator4")
    (Variables|Throwing|SetAimAngleDegrees (Math|Float|Clamp(Float) NewAimAngle (* _maxaimangledegrees -1.0) _maxaimangledegrees))))

(fn GetCurrentThrowDirection
  (return (Math|Vector|Normalize (Math|Vector|RotateVectorAroundAxis (Math|Vector|MakeVector 1.0 0.0 0.0) (Variables|Throwing|GetAimAngleDegrees) "0.000000,0.000000,1.000000"))))

(fn SetSpinAmount
  (params (NewSpinAmount :type Float%20%28double-precision%29))
  (if (Utilities|Enum|Equal(Enum) (Variables|Internal|GetCurrentRunPhase) "NewEnumerator4")
    (Variables|Throwing|SetSpinAmount (Math|Float|Clamp(Float) NewSpinAmount (* -1.0 (Variables|Controllers|GetMaxSpinAmount)) (Variables|Controllers|GetMaxSpinAmount)))))

(fn SetPowerAmount
  (params (NewPowerAmount :type Float%20%28double-precision%29))
  (Variables|Throwing|SetPowerAmount (Math|Float|Clamp(Float) NewPowerAmount (Variables|Throwing|GetMinPower) (Variables|Throwing|GetMaxPower))))

(fn StartChargingPower
  (if (Utilities|Enum|Equal(Enum) (Variables|Internal|GetCurrentRunPhase) "NewEnumerator4")
    (LevelFlow|EnterRunPhase "NewEnumerator11")
    (Variables|Throwing|SetbChargingPower true)
    (Variables|Throwing|SetPowerAmount (Variables|Throwing|GetMinPower))
    (Variables|Internal|SetPowerCharingDirection 1.0)))

(fn ReleasePowerandThrow
  (Variables|Throwing|SetbAimingActive false)
  (Variables|Throwing|SetbChargingPower false)
  (LevelFlow|RequestBallThrow (AimingandThrowing|GetCurrentThrowDirection) (* (Variables|Controllers|GetThrowStrength) (Variables|Throwing|GetPowerAmount))))

(fn HandlePowerMeter
  (if (Variables|Throwing|GetbChargingPower)
    (LocalVariables|SetNewPower (+ (* (Variables|Internal|GetDeltaSeconds) (Variables|Throwing|GetPowerChargeSpeed) (Variables|Internal|GetPowerCharingDirection)) (Variables|Throwing|GetPowerAmount)))
    (Utilities|FlowControl|Sequence
      (:then_0
        ;[0.15 0.15 0.15 0.5] Ping pong the meter
        (if (>= (LocalVariables|GetNewPower) (Variables|Throwing|GetMaxPower))
          (Variables|Internal|SetPowerCharingDirection -1.0)
          (elif (<= (LocalVariables|GetNewPower) (Variables|Throwing|GetMinPower))
            (Variables|Internal|SetPowerCharingDirection 1.0))))
      (:then_1
        (Variables|Throwing|SetPowerAmount (LocalVariables|GetNewPower))))))

(fn GetAvailableBallInstances
  (bind _ballsavailable (Default|GetAvailableBalls (Variables|/Game/Core/Framework/BP_BowlatroPlayerState.BP_BowlatroPlayerState_C|GetBPC_BallInventory (Variables|References|GetActivePlayerState))))
  (bind _output_get (LocalVariables|SetBallsAvailable _ballsavailable))
  (return _output_get))

(fn ClearLane
  (Utilities|FlowControl|Sequence
    (:then_0
      (Utilities|IsValid (Variables|References|GetActiveBallActor)
        (:Is%20Valid
          (Actor|DestroyActor (Variables|References|GetActiveBallActor))
          (Variables|References|SetActiveBallActor 0))))
    (:then_1
      (Utilities|IsValid (Variables|ThrowTracking|GetThrowManager)
        (:Is%20Valid
          (Utilities|Array|Clear (Variables|/Game/Core/Throw/BP_ThrowManager.BP_ThrowManager_C|GetActiveBallActors (Variables|ThrowTracking|GetThrowManager))))))
    (:then_2
      (Utilities|IsValid (Variables|References|GetPinRack)
        (:Is%20Valid
          (Default|ClearExistingPins (Variables|References|GetPinRack)))))))

(fn AimBall
  (params (ActionValue :type Vector%202D%20Structure))
  (bind _activeballactor (Variables|References|GetActiveBallActor))
  (bind _ballmesh (Variables|/Game/Core/Balls/BP_BowlingBallActor.BP_BowlingBallActor_C|GetBallMesh _activeballactor))
  (Variables|Throwing|SetBallAimLocation (Math|Vector|MakeVector (.x (Variables|Throwing|GetBallAimLocation)) (+ (.y (Variables|Throwing|GetBallAimLocation)) (* (.x ActionValue) 2.0)) (.z (Variables|Throwing|GetBallAimLocation))))
  (Variables|Throwing|SetbAimingActive true)
  (Physics|SetSimulatePhysics _ballmesh false)
  (Transformation|SetWorldRotation _ballmesh (Math|Rotator|FindLookatRotation (Transformation|GetWorldLocation _ballmesh) (Variables|Throwing|GetBallAimLocation)) false false)
  (Physics|SetSimulatePhysics _ballmesh true))

(fn MoveStartingBallLocation
  (params (ActionValue :type Vector%202D%20Structure))
  (bind _activeballactor (Variables|References|GetActiveBallActor))
  (bind _ballmesh (Variables|/Game/Core/Balls/BP_BowlingBallActor.BP_BowlingBallActor_C|GetBallMesh _activeballactor))
  (bind _ballmesh_2 (Variables|/Game/Core/Balls/BP_BowlingBallActor.BP_BowlingBallActor_C|GetBallMesh _activeballactor))
  (bind _returnvalue (Transformation|GetWorldLocation _ballmesh_2))
  (Physics|SetSimulatePhysics _ballmesh false)
  (Transformation|SetWorldLocation _ballmesh (Math|Vector|MakeVector (.x _returnvalue) (Math|Float|Min(Float) (Math|Float|Max(Float) (+ (.x ActionValue) (.y _returnvalue)) -51.0) 51.0) (.z _returnvalue)) false true)
  (Physics|SetSimulatePhysics _ballmesh true))
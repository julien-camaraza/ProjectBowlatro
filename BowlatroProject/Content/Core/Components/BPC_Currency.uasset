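; Currency component that tracks a Gold balance, with functions to add, check and spend it.
; AddGold is the shared mutator, clamping the balance at zero; SpendGold passes it a negated amount only if CanAfford succeeds, and returns success.
; AddLevelEndGold awards a base amount plus a bonus per remaining frame.
; A Source argument accompanies gold changes but does not yet affect the result.
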(event EventBeginPlay)

(event EventTick
  (params (DeltaSeconds :type Float%20%28single-precision%29)))

(fn AddGold
  (params (Amount :type Integer) (Source :type E_GoldSource%20Enum :default "NewEnumerator0"))
  ;[0.15 0.15 0.15 0.5] Basic for now, but should be easy to add something like "Gain 20% more gold from round end" if needed
  (bind _output_get (Variables|Default|SetGold (Math|Integer|Max(Integer) (+ (Variables|Default|GetGold) Amount))))
  (return _output_get))

(fn CanAfford
  (params (Cost :type Integer))
  (return (<= Cost (Variables|Default|GetGold))))

(fn SpendGold
  (params (Amount :type Integer) (Source :type E_GoldSource%20Enum :default "NewEnumerator5"))
  (if (CallFunction|CanAfford Amount)
    (CallFunction|AddGold (* Amount -1) Source)
    (return true)
    (else
      (return false))))

(fn AddLevelEndGold
  (params (BaseGoldForLevelEnd :type Integer) (GoldPerFrameRemaining :type Integer) (RemainingFrames :type Integer))
  (CallFunction|AddGold (+ BaseGoldForLevelEnd (* GoldPerFrameRemaining RemainingFrames)) "NewEnumerator0"))
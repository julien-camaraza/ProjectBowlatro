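; Actor component that holds the player's inventory of throwable balls and tracks which are used in the current level.
; InitializeStarterBalls rebuilds the instance array from starter definitions, giving each an index-based ID.
; GetAvailableBalls returns unused instances, while MarkBallUsed finds one by ID, flags it used and increments its throw count.
; MarkAllBallsUnused clears the used flags, preserving throw counts and permanent score and multiplier bonuses.
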(event EventBeginPlay)

(event EventTick
  (params (DeltaSeconds :type Float%20%28single-precision%29)))

(fn InitializeStarterBalls
  (Utilities|Array|Clear (Variables|Default|GetBallInstances))
  (for (_array_element _array_index) (Variables|Default|GetStarterBallDefs)
    (Utilities|Array|Add (Variables|Default|GetBallInstances) (Utilities|Struct|MakeS_BallInstance (Utilities|String|StringToName (Utilities|String|ToString(Text) (Utilities|Text|FormatText "Ball_{0}" _array_index))) _array_element))))

(fn GetAvailableBalls
  (for _array_element (Variables|Default|GetBallInstances)
    (if (not (.bUsedThisLevel (Utilities|Struct|BreakS_BallInstance _array_element)))
      (Utilities|Array|Add (LocalVariables|GetAvailableBalls) _array_element)))
  (return (LocalVariables|GetAvailableBalls)))

(fn MarkBallUsed
  (params (InstanceID :type Name))
  ;[0.15 0.15 0.15 0.5] Find the ball we threw by ID and override it in our array with new data
  (bind (_array_element _array_index) (Utilities|Array|ForEachLoopwithBreak (Variables|Default|GetBallInstances) :!label _label)
    (:LoopBody
      (if (== (.InstanceID (Utilities|Struct|BreakS_BallInstance _array_element)) InstanceID)
        (Utilities|Array|SetArrayElem (Variables|Default|GetBallInstances) _array_index (Utilities|Struct|MakeS_BallInstance (.InstanceID (Utilities|Struct|BreakS_BallInstance _array_element)) (.BallDef (Utilities|Struct|BreakS_BallInstance _array_element)) (.PermanentBaseScoreBonus (Utilities|Struct|BreakS_BallInstance _array_element)) (.PermanentMultiplierBonus (Utilities|Struct|BreakS_BallInstance _array_element)) (+ (.TimesThrown (Utilities|Struct|BreakS_BallInstance _array_element)) 1) true))
        (goto _label Break)))))

(fn MarkAllBallsUnused
  (bind (_array_element _array_index) (Utilities|Array|ForEachLoopwithBreak (Variables|Default|GetBallInstances))
    (:LoopBody
      (Utilities|Array|SetArrayElem (Variables|Default|GetBallInstances) _array_index (Utilities|Struct|MakeS_BallInstance (.InstanceID (Utilities|Struct|BreakS_BallInstance _array_element)) (.BallDef (Utilities|Struct|BreakS_BallInstance _array_element)) (.PermanentBaseScoreBonus (Utilities|Struct|BreakS_BallInstance _array_element)) (.PermanentMultiplierBonus (Utilities|Struct|BreakS_BallInstance _array_element)) (.TimesThrown (Utilities|Struct|BreakS_BallInstance _array_element)))))))
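; Component that applies perk and ball effects to the score of a bowling throw.
; ApplyScoreEffects runs pre-score effects from owned perks, then the ball, rounds additive times multiplier into the final score, then runs post-score effects.
; ApplyArrayOfEffects filters specs by trigger, constructs each logic class to modify the score context, and logs before/after score, multiplier or gold changes as score events for UI.
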(event EventBeginPlay)

(event EventTick
  (params (DeltaSeconds :type Float%20%28single-precision%29)))

(fn ApplyScoreEffects
  (params (ScoreContext :type S%20Score%20Context%20Structure) (ThrowResult :type S%20Throw%20Result%20Structure))
  (bind (_ballinstance _playerstate) (Utilities|Struct|BreakS_ThrowResult ThrowResult))
  (LocalVariables|SetPlayerState _playerstate)
  (LocalVariables|SetScoreContextModified ScoreContext)
  (LocalVariables|SetBallEffects (Variables|/Game/Data/PDA_BallDef.PDA_BallDef_C|GetGrantedEffects (.BallDef (Utilities|Struct|BreakS_BallInstance _ballinstance))))
  (Utilities|FlowControl|Sequence
    (:then_0
      ;[0.15 0.15 0.15 0.5] PRE SCORE:
      ; Go through all pre score effects and apply them.
      ;;[0.15 0.15 0.15 0.5] Effects in the perk system
      (for _array_element (Variables|/Game/Core/Components/BPC_PerkInventory.BPC_PerkInventory_C|GetOwnedPerks (Variables|/Game/Core/Framework/BP_BowlatroPlayerState.BP_BowlatroPlayerState_C|GetBPC_PerkInventory (LocalVariables|GetPlayerState)))
        (bind _modifiedscorecontext (CallFunction|ApplyArrayOfEffects (Variables|/Game/Data/Perks/PDA_PerkDef.PDA_PerkDef_C|GetGrantedEffects _array_element) "NewEnumerator9" (LocalVariables|GetScoreContextModified) ThrowResult))
        (LocalVariables|SetScoreContextModified _modifiedscorecontext))
      ;;[0.15 0.15 0.15 0.5] Effects on the ball
      (bind _modifiedscorecontext_2 (CallFunction|ApplyArrayOfEffects (LocalVariables|GetBallEffects) "NewEnumerator9" (LocalVariables|GetScoreContextModified) ThrowResult))
      (LocalVariables|SetScoreContextModified _modifiedscorecontext_2))
    (:then_1
      ;[0.15 0.15 0.15 0.5] CALCULATE FINAL SCORE:
      ; Get finalized score. This will eventually want to be ceremonalized.
      (LocalVariables|SetScoreContextModified (Utilities|Struct|MakeS_ScoreContext (.AdditiveScore (Utilities|Struct|BreakS_ScoreContext (LocalVariables|GetScoreContextModified))) (.Multiplier (Utilities|Struct|BreakS_ScoreContext (LocalVariables|GetScoreContextModified))) (.BaseBallScore (Utilities|Struct|BreakS_ScoreContext (LocalVariables|GetScoreContextModified))) (.PinScore (Utilities|Struct|BreakS_ScoreContext (LocalVariables|GetScoreContextModified))) (.BonusBallScore (Utilities|Struct|BreakS_ScoreContext (LocalVariables|GetScoreContextModified))) (.KnockedPinCount (Utilities|Struct|BreakS_ScoreContext (LocalVariables|GetScoreContextModified))) (.bAllPinsCleared (Utilities|Struct|BreakS_ScoreContext (LocalVariables|GetScoreContextModified))) (.bWasSplit (Utilities|Struct|BreakS_ScoreContext (LocalVariables|GetScoreContextModified))) (.ScoreEvents (Utilities|Struct|BreakS_ScoreContext (LocalVariables|GetScoreContextModified))) (Math|Float|Round (* (.AdditiveScore (Utilities|Struct|BreakS_ScoreContext (LocalVariables|GetScoreContextModified))) (.Multiplier (Utilities|Struct|BreakS_ScoreContext (LocalVariables|GetScoreContextModified))))))))
    (:then_2
      ;[0.15 0.15 0.15 0.5] POST SCORE:
      ; Go through all post score effects and apply them.
      ;;[0.15 0.15 0.15 0.5] Effects in the perk system
      (for _array_element_2 (Variables|/Game/Core/Components/BPC_PerkInventory.BPC_PerkInventory_C|GetOwnedPerks (Variables|/Game/Core/Framework/BP_BowlatroPlayerState.BP_BowlatroPlayerState_C|GetBPC_PerkInventory (LocalVariables|GetPlayerState)))
        (bind _modifiedscorecontext_3 (CallFunction|ApplyArrayOfEffects (Variables|/Game/Data/Perks/PDA_PerkDef.PDA_PerkDef_C|GetGrantedEffects _array_element_2) "NewEnumerator10" (LocalVariables|GetScoreContextModified) ThrowResult))
        (LocalVariables|SetScoreContextModified _modifiedscorecontext_3))
      (bind _modifiedscorecontext_4 (CallFunction|ApplyArrayOfEffects (LocalVariables|GetBallEffects) "NewEnumerator10" (LocalVariables|GetScoreContextModified) ThrowResult))
      (bind _output_get (LocalVariables|SetScoreContextModified _modifiedscorecontext_4))
      (return _output_get))))

(fn ApplyArrayOfEffects
  (params (ArrayOfEffects :type Array%20of%20S%20Effect%20Spec%20Structures) (EffectTriggerRequired :type E_EffectTrigger%20Enum :default "NewEnumerator0") (ScoreContextPreModified :type S%20Score%20Context%20Structure) (ThrowResult :type S%20Throw%20Result%20Structure))
  (LocalVariables|SetScoreContextModified ScoreContextPreModified)
  (LocalVariables|SetPlayerCurrencyRef (Variables|/Game/Core/Framework/BP_BowlatroPlayerState.BP_BowlatroPlayerState_C|GetBPC_Currency (Utilities|Struct|BreakS_ThrowResult ThrowResult)))
  ;[0.15 0.15 0.15 0.5] We want this to be as modular as possible, so with any array of effects we pass in, we check if we're in the right trigger and then modify as needed
  (for _array_element ArrayOfEffects
    (LocalVariables|SetLoop_CurrentEffectSpec _array_element)
    (LocalVariables|SetLoop_ScoreContextPreModified (LocalVariables|GetScoreContextModified))
    (LocalVariables|SetLoop_AdditivePreModified (.AdditiveScore (Utilities|Struct|BreakS_ScoreContext (LocalVariables|GetScoreContextModified))))
    (LocalVariables|SetLoop_MultiplierPreModified (.Multiplier (Utilities|Struct|BreakS_ScoreContext (LocalVariables|GetScoreContextModified))))
    (LocalVariables|SetLoop_GoldPreModified (Variables|/Game/Core/Components/BPC_Currency.BPC_Currency_C|GetGold (LocalVariables|GetPlayerCurrencyRef)))
    (if (Utilities|Enum|Equal(Enum) EffectTriggerRequired (.EffectTrigger (Utilities|Struct|BreakS_EffectSpec (LocalVariables|GetLoop_CurrentEffectSpec))))
      (bind _returnvalue (Game|ConstructObjectfromClass (.EffectLogic (Utilities|Struct|BreakS_EffectSpec (LocalVariables|GetLoop_CurrentEffectSpec))))) ; This gets deleted when nothing else references it, so no memory leak
      (bind _modifiedscorecontext (Default|ModifyScore _returnvalue (LocalVariables|GetScoreContextModified) ThrowResult (.MagnitudeInt (Utilities|Struct|BreakS_EffectSpec (LocalVariables|GetLoop_CurrentEffectSpec))) (.MagnitudeFloat (Utilities|Struct|BreakS_EffectSpec (LocalVariables|GetLoop_CurrentEffectSpec)))))
      (bind _output_get (LocalVariables|SetScoreContextModified _modifiedscorecontext))
      ;[0.15 0.15 0.15 0.5] create context for UI
      (LocalVariables|SetLoop_AdditivePostModified (.AdditiveScore (Utilities|Struct|BreakS_ScoreContext _output_get)))
      (LocalVariables|SetLoop_MultiplierPostModified (.Multiplier (Utilities|Struct|BreakS_ScoreContext _output_get)))
      (LocalVariables|SetLoop_GoldPostModified (Variables|/Game/Core/Components/BPC_Currency.BPC_Currency_C|GetGold (LocalVariables|GetPlayerCurrencyRef)))
      (LocalVariables|SetLoop_AdditiveDelta (- (LocalVariables|GetLoop_AdditivePostModified) (LocalVariables|GetLoop_AdditivePreModified)))
      (LocalVariables|SetLoop_MultiplierDelta (- (LocalVariables|GetLoop_MultiplierPostModified) (LocalVariables|GetLoop_MultiplierPreModified)))
      (LocalVariables|SetLoop_GoldDelta (- (LocalVariables|GetLoop_GoldPostModified) (LocalVariables|GetLoop_GoldPreModified)))
      (LocalVariables|SetLoop_ScoreEvents (Utilities|Struct|BreakS_ScoreContext (LocalVariables|GetScoreContextModified)))
      (Utilities|FlowControl|Sequence
        (:then_0
          ;[0.15 0.15 0.15 0.5] This could be a select node, but I think it's more clear if each one uses it's own logic. It also means we can do more custom casing in the future.
          (switch Utilities|FlowControl|Switch|SwitchonE_ScoreEventType (Utilities|Struct|BreakS_EffectSpec (LocalVariables|GetLoop_CurrentEffectSpec))
            (:NewEnumerator0
              (LocalVariables|SetLoop_NewScoreEvent (Utilities|Struct|MakeS_ScoreEvent (.EffectName (Utilities|Struct|BreakS_EffectSpec (LocalVariables|GetLoop_CurrentEffectSpec))) (.PresentationType (Utilities|Struct|BreakS_EffectSpec (LocalVariables|GetLoop_CurrentEffectSpec))) (Math|Conversions|ToFloat(Integer) (LocalVariables|GetLoop_AdditiveDelta)))))
            (:NewEnumerator1
              (LocalVariables|SetLoop_NewScoreEvent (Utilities|Struct|MakeS_ScoreEvent (.EffectName (Utilities|Struct|BreakS_EffectSpec (LocalVariables|GetLoop_CurrentEffectSpec))) (.PresentationType (Utilities|Struct|BreakS_EffectSpec (LocalVariables|GetLoop_CurrentEffectSpec))) (LocalVariables|GetLoop_MultiplierDelta))))
            (:NewEnumerator2
              (LocalVariables|SetLoop_NewScoreEvent (Utilities|Struct|MakeS_ScoreEvent (.EffectName (Utilities|Struct|BreakS_EffectSpec (LocalVariables|GetLoop_CurrentEffectSpec))) (.PresentationType (Utilities|Struct|BreakS_EffectSpec (LocalVariables|GetLoop_CurrentEffectSpec))) (Math|Float|SafeDivide (LocalVariables|GetLoop_MultiplierPostModified) (LocalVariables|GetLoop_MultiplierPreModified)))))
            (:NewEnumerator3
              (LocalVariables|SetLoop_NewScoreEvent (Utilities|Struct|MakeS_ScoreEvent (.EffectName (Utilities|Struct|BreakS_EffectSpec (LocalVariables|GetLoop_CurrentEffectSpec))) (.PresentationType (Utilities|Struct|BreakS_EffectSpec (LocalVariables|GetLoop_CurrentEffectSpec))) (Math|Conversions|ToFloat(Integer) (LocalVariables|GetLoop_GoldDelta)))))
            (:NewEnumerator4
              (LocalVariables|SetLoop_NewScoreEvent (Utilities|Struct|MakeS_ScoreEvent (.EffectName (Utilities|Struct|BreakS_EffectSpec (LocalVariables|GetLoop_CurrentEffectSpec))) (.PresentationType (Utilities|Struct|BreakS_EffectSpec (LocalVariables|GetLoop_CurrentEffectSpec))) (Math|Float|SafeDivide (Math|Conversions|ToFloat(Integer) (LocalVariables|GetLoop_GoldPostModified)) (Math|Conversions|ToFloat(Integer) (LocalVariables|GetLoop_GoldPreModified))))))))
        (:then_1
          ;;[0.15 0.15 0.15 0.5] Update score context with the new event we've made
          (Utilities|Array|Add (LocalVariables|GetLoop_ScoreEvents) (LocalVariables|GetLoop_NewScoreEvent))
          (LocalVariables|SetScoreContextModified (Utilities|Struct|MakeS_ScoreContext (.AdditiveScore (Utilities|Struct|BreakS_ScoreContext (LocalVariables|GetScoreContextModified))) (.Multiplier (Utilities|Struct|BreakS_ScoreContext (LocalVariables|GetScoreContextModified))) (.BaseBallScore (Utilities|Struct|BreakS_ScoreContext (LocalVariables|GetScoreContextModified))) (.PinScore (Utilities|Struct|BreakS_ScoreContext (LocalVariables|GetScoreContextModified))) (.BonusBallScore (Utilities|Struct|BreakS_ScoreContext (LocalVariables|GetScoreContextModified))) (.KnockedPinCount (Utilities|Struct|BreakS_ScoreContext (LocalVariables|GetScoreContextModified))) (.bAllPinsCleared (Utilities|Struct|BreakS_ScoreContext (LocalVariables|GetScoreContextModified))) (.bWasSplit (Utilities|Struct|BreakS_ScoreContext (LocalVariables|GetScoreContextModified))) (LocalVariables|GetLoop_ScoreEvents) (.FinalScore (Utilities|Struct|BreakS_ScoreContext (LocalVariables|GetScoreContextModified)))))))))
  (return (LocalVariables|GetScoreContextModified)))
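; Score resolver component that turns a bowling throw result into a score context with a final score.
; CalculateThrowScore adds the ball's base score and permanent bonus to a per-pin score for pins knocked that throw.
; Each non-zero part logs a named score event.
; The sum is scaled by the ball's permanent multiplier bonus, rounded, and returned with the breakdown, events and all-pins-cleared flag.
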(event EventBeginPlay)

(event EventTick
  (params (DeltaSeconds :type Float%20%28single-precision%29)))

(fn CalculateThrowScore
  (params (ThrowResult :type S%20Throw%20Result%20Structure))
  (bind _ballinstance (Utilities|Struct|BreakS_ThrowResult ThrowResult))
  (bind _pinsknocked_thisthrow (Utilities|Struct|BreakS_ThrowResult ThrowResult))
  (bind (_balldef _permanentbasescorebonus) (Utilities|Struct|BreakS_BallInstance _ballinstance))
  ;[0.15 0.15 0.15 0.5] Ball Score
  (bind _output_get (LocalVariables|SetBaseScore (+ (Variables|/Game/Data/PDA_BallDef.PDA_BallDef_C|GetBaseScore _balldef) _permanentbasescorebonus)))
  (if (!= _output_get 0)
    (Utilities|Array|Add (LocalVariables|GetScoreEvents) (Utilities|Struct|MakeS_ScoreEvent (Variables|/Game/Data/PDA_BallDef.PDA_BallDef_C|GetDisplayName _balldef) "NewEnumerator0" (Math|Conversions|ToFloat(Integer) (LocalVariables|GetBaseScore)))))
  ;[0.15 0.15 0.15 0.5] Pin Score
  (bind _output_get_2 (LocalVariables|SetPinScore (* (Variables|Default|GetScorePerPin) _pinsknocked_thisthrow)))
  (if (!= _output_get_2 0)
    (Utilities|Array|Add (LocalVariables|GetScoreEvents) (Utilities|Struct|MakeS_ScoreEvent (Utilities|Text|FormatText "{0} per Pin ({1})" (Variables|Default|GetScorePerPin) _pinsknocked_thisthrow) "NewEnumerator0" (Math|Conversions|ToFloat(Integer) (LocalVariables|GetPinScore)))))
  (LocalVariables|SetMultiplier (+ 1.0 (.PermanentMultiplierBonus (Utilities|Struct|BreakS_BallInstance (.BallInstance (Utilities|Struct|BreakS_ThrowResult ThrowResult))))))
  (LocalVariables|SetAdditiveScore (+ (LocalVariables|GetBaseScore) (LocalVariables|GetPinScore)))
  (LocalVariables|SetFinalScore (Math|Float|Round (* (LocalVariables|GetMultiplier) (LocalVariables|GetAdditiveScore))))
  (return (Utilities|Struct|MakeS_ScoreContext (LocalVariables|GetAdditiveScore) (LocalVariables|GetMultiplier) (LocalVariables|GetBaseScore) (LocalVariables|GetPinScore) 0 0 (.bClearedAllPins (Utilities|Struct|BreakS_ThrowResult ThrowResult)) false (LocalVariables|GetScoreEvents) (LocalVariables|GetFinalScore))))
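; Game mode for Bowlatro that drives a bowling run through rounds, level completion and the shop.
; On BeginPlay it spawns the RunManager, finds the LaneManager, starts the run and binds round success and failure events.
; Success grants fixed gold, changes run phase, opens a debug shop and advances the round; failure is still empty.
; Separate functions start the next round and award gold for remaining frames.
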(event Custom|HandleLevelCompleted
  ;[0.15 0.15 0.15 0.5] Handle level completed
  (Default|AddGold (Variables|/Game/Core/Framework/BP_BowlatroPlayerState.BP_BowlatroPlayerState_C|GetBPC_Currency (Variables|References|GetPlayerState)) 10 "NewEnumerator0")
  (Default|EnterRunPhase (Variables|References|GetLaneManager) "NewEnumerator8")
  (Default|GenerateDebugShop (Variables|References|GetRunManager))
  (Default|OpenShop (Variables|References|GetPlayerController))
  (Default|AdvanceRound (Variables|References|GetRunManager)))

(event Custom|HandleLevelFailed
  ;[0.15 0.15 0.15 0.5] Handle level failed
)

(event EventBeginPlay
  (CallFunction|InitalizeSecondaryActors)
  (CallFunction|StartRun)
  (Utilities|FlowControl|Sequence
    (:then_0
      ;[0.15 0.15 0.15 0.5] Handle level completed
      (EventDispatchers|BindEventtoOnRoundCompletedSuccesfully (Variables|References|GetLaneManager) (delegate Custom|HandleLevelCompleted)))
    (:then_1
      ;[0.15 0.15 0.15 0.5] Handle level failed
      (EventDispatchers|BindEventtoOnRoundFailed (Variables|References|GetLaneManager) (delegate Custom|HandleLevelFailed)))))

(event EventTick
  (params (DeltaSeconds :type Float%20%28single-precision%29)))

(fn ConstructionScript)

(fn InitalizeSecondaryActors
  (bind _returnvalue (Game|SpawnActorfromClass (Variables|Classes|GetRunManagerClass) (Math|Transform|MakeTransform "0, 0, 0") "Undefined" "MultiplyWithRoot" 0 0))
  (Variables|References|SetRunManager _returnvalue)
  (Variables|References|SetPlayerController (.AsBP%20Bowlatro%20Player%20Controller (Utilities|Casting|CastToBP_BowlatroPlayerController (Game|GetPlayerController 0))))
  (Variables|/Game/Core/Framework/BP_BowlatroPlayerController.BP_BowlatroPlayerController_C|SetRunManager (Variables|References|GetPlayerController) (Variables|References|GetRunManager))
  (bind _outactors (Actor|GetAllActorsOfClass "/Game/Core/Lane/BP_LaneManager.BP_LaneManager_C"))
  (Variables|References|SetLaneManager (Utilities|Array|Get(acopy) _outactors)))

(fn ContinueRun
  (bind _runmanager (Variables|References|GetRunManager))
  (Default|StartRound (Variables|References|GetLaneManager) (Default|GetCurrentRound _runmanager) (Default|GetCurrentStage _runmanager)))

(fn StartRun
  (bind _runmanager (Variables|References|GetRunManager))
  ;[0.15 0.15 0.15 0.5] Start Run
  (bind _output_get (Variables|References|SetPlayerState (.AsBP%20Bowlatro%20Player%20State (Utilities|Casting|CastToBP_BowlatroPlayerState (Variables|/Script/Engine.Controller|GetPlayerState (Game|GetPlayerController 0))))))
  (Default|StartRun _output_get)
  (Default|StartRun (Variables|References|GetRunManager))
  (Default|StartStage (Variables|References|GetLaneManager) (Default|GetCurrentStage _runmanager) (Default|GetCurrentRound _runmanager)))

(fn TriggerLevelEndGoldGain
  (params (PlayerStateToTriggerOn :type BP%20Bowlatro%20Player%20State%20Object%20Reference) (RemainingFrames :type Integer))
  (bind _runmanager (Variables|References|GetRunManager))
  (Default|AddLevelEndGold (Variables|/Game/Core/Framework/BP_BowlatroPlayerState.BP_BowlatroPlayerState_C|GetBPC_Currency PlayerStateToTriggerOn) (Default|GetGoldGainPerLevel _runmanager) (Default|GetGoldPerRemainingFrame _runmanager) RemainingFrames))
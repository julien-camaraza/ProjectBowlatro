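; Player controller for Bowlatro that turns keyboard input into bowling throw controls on the lane.
; On BeginPlay it caches the first BP_LaneManager in the world.
; Space starts power charging and releases the throw, while A/D or arrow keys and Q/E set aim and spin directions.
; Tick scales those directions by speed and delta time to update the lane manager's aim angle and spin, a hard-coded stopgap until a proper input system.
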(event EventBeginPlay
  (|CallParentFunction)
  (bind _outactors (Actor|GetAllActorsOfClass "/Game/Core/Lane/BP_LaneManager.BP_LaneManager_C"))
  (Variables|References|SetLaneManager (Utilities|Array|Get(acopy) _outactors)))

(event EventTick
  (params (DeltaSeconds :type Float%20%28single-precision%29))
  (bind _lanemanager (Variables|References|GetLaneManager))
  (bind _lanemanager_2 (Variables|References|GetLaneManager))
  ;[0.15 0.15 0.15 0.5] TO DO: Replace this with a robust input system
  (Variables|Internal|SetDeltaSeconds DeltaSeconds) ; I don't love doing this on tick, but I figure it's better than having messy script at least for now
  (Utilities|FlowControl|Sequence
    (:then_0
      (if (Utilities|IsValid (Variables|References|GetLaneManager)) ; Stuff dependent on lane manager
        (Utilities|FlowControl|Sequence
          (:then_0
            ;;[0.15 0.15 0.15 0.5] Adjust aim angle
            (if (!= (Variables|Internal|GetAimInputDirection) 0.0)
              (Default|SetAimAngle _lanemanager_2 (+ (Variables|/Game/Core/Lane/BP_LaneManager.BP_LaneManager_C|GetAimAngleDegrees _lanemanager_2) (* (Variables|Controllers|GetAimTurnSpeedDegreesPerSecond) (Variables|Internal|GetAimInputDirection) (Variables|Internal|GetDeltaSeconds))))))
          (:then_1
            ;;[0.15 0.15 0.15 0.5] Adjust aim angle
            (if (!= (Variables|Internal|GetSpinInputDirection) 0.0)
              (Default|SetSpinAmount _lanemanager (+ (Variables|/Game/Core/Lane/BP_LaneManager.BP_LaneManager_C|GetSpinAmount _lanemanager) (* (Variables|Controllers|GetSpinChangeSpeedPerSecond) (Variables|Internal|GetDeltaSeconds) (Variables|Internal|GetSpinInputDirection)))))))))))

(event Input|KeyboardEvents|SpaceBar
  (params (Key :type Key%20Structure :default "None"))
  (bind _lanemanager (Variables|References|GetLaneManager))
  ;[0.15 0.15 0.15 0.5] TO DO: Replace this with a robust input system
  (:Pressed
    (Default|StartChargingPower _lanemanager))
  (:Released
    (Default|ReleasePowerandThrow _lanemanager)))

(event Input|KeyboardEvents|A
  (params (Key :type Key%20Structure :default "None"))
  ;[0.15 0.15 0.15 0.5] TO DO: Replace this with a robust input system
  ;;[0.15 0.15 0.15 0.5] Set aim change per tick
  (:Pressed
    (Variables|Internal|SetAimInputDirection -1.0))
  (:Released
    (Variables|Internal|SetAimInputDirection 0.0)))

(event Input|KeyboardEvents|Left
  (params (Key :type Key%20Structure :default "None"))
  ;[0.15 0.15 0.15 0.5] TO DO: Replace this with a robust input system
  ;;[0.15 0.15 0.15 0.5] Set aim change per tick
  (:Pressed
    (Variables|Internal|SetAimInputDirection -1.0))
  (:Released
    (Variables|Internal|SetAimInputDirection 0.0)))

(event Input|KeyboardEvents|D
  (params (Key :type Key%20Structure :default "None"))
  ;[0.15 0.15 0.15 0.5] TO DO: Replace this with a robust input system
  ;;[0.15 0.15 0.15 0.5] Set aim change per tick
  (:Pressed
    (Variables|Internal|SetAimInputDirection 1.0))
  (:Released
    (Variables|Internal|SetAimInputDirection 0.0)))

(event Input|KeyboardEvents|Right
  (params (Key :type Key%20Structure :default "None"))
  ;[0.15 0.15 0.15 0.5] TO DO: Replace this with a robust input system
  ;;[0.15 0.15 0.15 0.5] Set aim change per tick
  (:Pressed
    (Variables|Internal|SetAimInputDirection 1.0))
  (:Released
    (Variables|Internal|SetAimInputDirection 0.0)))

(event Input|KeyboardEvents|Q
  (params (Key :type Key%20Structure :default "None"))
  ;[0.15 0.15 0.15 0.5] TO DO: Replace this with a robust input system
  ;;[0.15 0.15 0.15 0.5] Set spin change per tick
  (:Pressed
    (Variables|Internal|SetSpinInputDirection -1.0))
  (:Released
    (Variables|Internal|SetSpinInputDirection 0.0)))

(event Input|KeyboardEvents|E
  (params (Key :type Key%20Structure :default "None"))
  ;[0.15 0.15 0.15 0.5] TO DO: Replace this with a robust input system
  ;;[0.15 0.15 0.15 0.5] Set spin change per tick
  (:Pressed
    (Variables|Internal|SetSpinInputDirection 1.0))
  (:Released
    (Variables|Internal|SetSpinInputDirection 0.0)))

(fn ConstructionScript
  (|CallParentFunction))